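; Unit component that tracks class, level, XP and per-level spell slots for the turn-based tile toolkit.
; BeginPlay calls Rest, which dispatches on class; only Wizard is handled, using a hard-coded 20-level slot table.
; At level 1, Wizard also adds the first spell to the owner's BP_AbilitySystem.
; XPGain recursively carries surplus XP through level-ups without refreshing slots, which waits for Rest.
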(event `self.ReceiveBeginPlay`
  (`self.Rest`))

(fn `AddAbility`
  (params (AbilityToCheck :type "/Game/AdvancedTurnBasedTileToolkit/Core/Abilities/BP_Ability Class Reference"))
  (`KismetArrayLibrary.Array_Add` (`/Game/AdvancedTurnBasedTileToolkit/Core/Units/BP_AbilitySystem.Abilities` (`Actor.GetComponentByClass` (`self.GetOwner`) "/Game/AdvancedTurnBasedTileToolkit/Core/Units/BP_AbilitySystem.BP_AbilitySystem_C")) AbilityToCheck))

(fn `Rest`
  (switch `string` (`self.MyClass`)
    (:`Wizard`
      (`self.Wizard`))))

(fn `Wizard`
  (switch `int` (`self.Level`)
    (:`1`
      (set `self.1stLevel` 2)
      (`self.AddAbility` (`|GetArrayItem` (`self.Spells`)))
      (return))
    (:`2`
      (set `self.1stLevel` 3)
      (set `self.2ndLevel` 2))
    (:`3`
      (set `self.1stLevel` 4)
      (set `self.2ndLevel` 3))
    (:`4`
      (set `self.1stLevel` 4)
      (set `self.2ndLevel` 3))
    (:`5`
      (set `self.1stLevel` 4)
      (set `self.2ndLevel` 3)
      (set `self.3rdLevel` 2))
    (:`6`
      (set `self.1stLevel` 4)
      (set `self.2ndLevel` 3)
      (set `self.3rdLevel` 3))
    (:`7`
      (set `self.1stLevel` 4)
      (set `self.2ndLevel` 3)
      (set `self.3rdLevel` 3)
      (set `self.4thLevel` 1))
    (:`8`
      (set `self.1stLevel` 4)
      (set `self.2ndLevel` 3)
      (set `self.3rdLevel` 3)
      (set `self.4thLevel` 2))
    (:`9`
      (set `self.1stLevel` 4)
      (set `self.2ndLevel` 3)
      (set `self.3rdLevel` 3)
      (set `self.4thLevel` 3)
      (set `self.5thLevel` 1))
    (:`10`
      (set `self.1stLevel` 4)
      (set `self.2ndLevel` 3)
      (set `self.3rdLevel` 3)
      (set `self.4thLevel` 3)
      (set `self.5thLevel` 2))
    (:`11`
      (set `self.1stLevel` 4)
      (set `self.2ndLevel` 3)
      (set `self.3rdLevel` 3)
      (set `self.4thLevel` 3)
      (set `self.5thLevel` 2)
      (set `self.6thLevel` 1))
    (:`12`
      (set `self.1stLevel` 4)
      (set `self.2ndLevel` 3)
      (set `self.3rdLevel` 3)
      (set `self.4thLevel` 3)
      (set `self.5thLevel` 2)
      (set `self.6thLevel` 1))
    (:`13`
      (set `self.1stLevel` 4)
      (set `self.2ndLevel` 3)
      (set `self.3rdLevel` 3)
      (set `self.4thLevel` 3)
      (set `self.5thLevel` 2)
      (set `self.6thLevel` 1)
      (set `self.7thLevel` 1))
    (:`14`
      (set `self.1stLevel` 4)
      (set `self.2ndLevel` 3)
      (set `self.3rdLevel` 3)
      (set `self.4thLevel` 3)
      (set `self.5thLevel` 2)
      (set `self.6thLevel` 1)
      (set `self.7thLevel` 1))
    (:`15`
      (set `self.1stLevel` 4)
      (set `self.2ndLevel` 3)
      (set `self.3rdLevel` 3)
      (set `self.4thLevel` 3)
      (set `self.5thLevel` 2)
      (set `self.6thLevel` 1)
      (set `self.7thLevel` 1)
      (set `self.8thLevel` 1))
    (:`16`
      (set `self.1stLevel` 4)
      (set `self.2ndLevel` 3)
      (set `self.3rdLevel` 3)
      (set `self.4thLevel` 3)
      (set `self.5thLevel` 2)
      (set `self.6thLevel` 1)
      (set `self.7thLevel` 1)
      (set `self.8thLevel` 1))
    (:`17`
      (set `self.1stLevel` 4)
      (set `self.2ndLevel` 3)
      (set `self.3rdLevel` 3)
      (set `self.4thLevel` 3)
      (set `self.5thLevel` 2)
      (set `self.6thLevel` 1)
      (set `self.7thLevel` 1)
      (set `self.8thLevel` 1)
      (set `self.9thLevel` 1))
    (:`18`
      (set `self.1stLevel` 4)
      (set `self.2ndLevel` 3)
      (set `self.3rdLevel` 3)
      (set `self.4thLevel` 3)
      (set `self.5thLevel` 3)
      (set `self.6thLevel` 1)
      (set `self.7thLevel` 1)
      (set `self.8thLevel` 1)
      (set `self.9thLevel` 1))
    (:`19`
      (set `self.1stLevel` 4)
      (set `self.2ndLevel` 3)
      (set `self.3rdLevel` 3)
      (set `self.4thLevel` 3)
      (set `self.5thLevel` 3)
      (set `self.6thLevel` 2)
      (set `self.7thLevel` 1)
      (set `self.8thLevel` 1)
      (set `self.9thLevel` 1))
    (:`20`
      (set `self.1stLevel` 4)
      (set `self.2ndLevel` 3)
      (set `self.3rdLevel` 3)
      (set `self.4thLevel` 3)
      (set `self.5thLevel` 3)
      (set `self.6thLevel` 2)
      (set `self.7thLevel` 2)
      (set `self.8thLevel` 1)
      (set `self.9thLevel` 1))))

(fn `XPGain`
  (params (XPGained :type "Float (double-precision)"))
  (bind _output_get (set `self.CurrentXP` (+ XPGained (`self.CurrentXP`))))
  (if (>= _output_get (`self.LvlUpXp`))
    (set `self.Level` (+ (`self.Level`) 1))
    (set `self.CurrentXP` (- (`self.CurrentXP`) (`self.LvlUpXp`)))
    (`self.XPGain` 0.0)
    (else
      (return))))