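; Boss attack ability for the turn-based tile toolkit, extending a parent attack ability with a hit effect.
; On AttackHit it looks up the unit at the target index in the grid manager and attaches the P_ky_hit emitter to it, then runs the parent hit logic.
; Ability execution and construction only forward to the parent.
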(event `self.AttackHit`
  (`GameplayStatics.SpawnEmitterAttached` "/Game/AdvancedMagicFX12/particles/P_ky_hit.P_ky_hit" (`/Game/AdvancedTurnBasedTileToolkit/Core/Grid/BP_GridActor.SceneComponent` (`BlueprintMapLibrary.Map_Find` (`/Game/AdvancedTurnBasedTileToolkit/Core/Grid/BP_GridManager.GridUnits` (`self.GridManagerRef`)) (`self.TargetIndex`))))
  (`parent.AttackHit`))

(fn `ExecuteAbility`
  (params (TargetIndex :type Integer))
  (returns (bSuccess :type Boolean))
  (bind _bsuccess (`parent.ExecuteAbility` TargetIndex))
  (return _bsuccess))

(fn `UserConstructionScript`
  (`parent.UserConstructionScript`))