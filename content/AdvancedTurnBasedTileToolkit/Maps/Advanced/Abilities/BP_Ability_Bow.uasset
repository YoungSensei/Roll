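; Bow ability Blueprint for the Advanced Turn Based Tile Toolkit that presents an Elven Longbow, described as firing an arrow at an enemy.
; It overrides GetDescription to build the description text, inserting the minimum and maximum of DamageRange into the wording.
; The event graph holds only disabled stubs and the construction script just calls the parent, so the file itself contains no firing or damage logic.
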(fn `GetDescription`
  (returns (Description :type Text))
  (bind (_damagerange_min _damagerange_max) (break `/Game/AdvancedTurnBasedTileToolkit/Maps/Advanced/Abilities/FDamageRange` (`self.DamageRange`)))
  (return (`KismetTextLibrary.Conv_StringToText` (`KismetStringLibrary.Concat_StrStr` (`KismetTextLibrary.Conv_TextToString` "Elven Longbow: \n") (`KismetTextLibrary.Conv_TextToString` "Fire an arrow for ") "" (`KismetStringLibrary.Conv_IntToString` _damagerange_min) " - " (`KismetStringLibrary.Conv_IntToString` _damagerange_max) (`KismetTextLibrary.Conv_TextToString` " points of damage at \nan enemy. May your aim be true..")))))

(fn `UserConstructionScript`
  (`parent.UserConstructionScript`))