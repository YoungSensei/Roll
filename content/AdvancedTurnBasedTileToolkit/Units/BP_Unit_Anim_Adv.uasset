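; Animated unit Blueprint in the Advanced Turn Based Tile Toolkit that picks its visible body by faction.
; On BeginPlay it reads its faction, showing Mesh and hiding Skeleton for the first faction value, and the reverse for any other.
; The parent BeginPlay call is disabled, so only this visibility switch runs there, while the construction script just defers to the parent.
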(event `self.ReceiveBeginPlay`
  (bind _faction (`/Game/AdvancedTurnBasedTileToolkit/Core/BPI_Initiative.GetFaction`))
  (if (`|EnumEquality` _faction "NewEnumerator0")
    (`SceneComponent.SetHiddenInGame` (`self.Skeleton`) true false)
    (`SceneComponent.SetHiddenInGame` (`self.Mesh`) false false)
    (else
      (`SceneComponent.SetHiddenInGame` (`self.Skeleton`) false false)
      (`SceneComponent.SetHiddenInGame` (`self.Mesh`) true false))))

(fn `UserConstructionScript`
  (`parent.UserConstructionScript`))