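; BPA_Item_Book is a pickup book that teaches a talent to the hero who uses it.
; On overlap with a talent-interface hero it refreshes and shows its tooltip widget and, if the hero's level meets the requirement, registers itself as the interactable item.
; ItemUse checks the talent isn't already learned, then once grants it without spending points through the interface, spawns a fire effect and expires.
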(event `/Game/TalentTreeBuilder/Blueprints/I_InteractableItem.Item_Use`
  (params (UserSelfNode :type "Actor Object Reference"))
  (`/Engine/EditorBlueprintResources/StandardMacros.IsValid` UserSelfNode
    (:`Is Valid`
      ;[1 1 1] Don't learn Talent if already has it
      (bind (_fail _hastargetprogress) (`/Game/TalentTreeBuilder/Blueprints/LibFuncTalentSystem.CheckTalent_TargetProgress_ByNameID` UserSelfNode (`self.UnlockTalentIndex`) 1))
      (if (not _hastargetprogress)
        ;[1 1 1] Call Event LearnTalent via Interface
        (`/Engine/EditorBlueprintResources/StandardMacros.DoOnce` false
          (:`Completed`
            (message `/Game/TalentTreeBuilder/Blueprints/I_HeroTalents.LearnTalent_ByDataTableID` UserSelfNode (`self.UnlockTalentIndex`) true)
            (`|SpawnActorFromClass` "/Game/TalentTreeBuilder/Blueprints/BonusExamples/BPA_Effect.BPA_Effect_C" (`KismetMathLibrary.MakeTransform` (`self.K2_GetActorLocation`)) "AlwaysSpawn" "OverrideRootScale" null "/Game/TalentTreeBuilder/UnnecessaryContent/Particles/FX_Ambient/Fire/P_Fire_Book.P_Fire_Book" 2.0)
            (`self.SetLifeSpan` 0.1)))))))

(event `self.Collision.OnComponentBeginOverlap`
  (params (OverlappedComponent :type "PrimitiveComponent Object Reference") (OtherActor :type "Actor Object Reference") (OtherComp :type "PrimitiveComponent Object Reference") (OtherBodyIndex :type Integer) (bFromSweep :type Boolean) (SweepResult :type "HitResult Structure (by ref)"))
  (`/Game/TalentTreeBuilder/Blueprints/LibMacroTalentSystem.CheckHeroTalentInterface` OtherActor
    (:`true`
      (bind _currentlevel (message `/Game/TalentTreeBuilder/Blueprints/I_HeroTalents.GetHero_Level` OtherActor))
      (bind _returnvalue (>= _currentlevel (`self.Required_Level`)))
      (`/Game/TalentTreeBuilder/UI/BonusWidgets/W_ItemTooltip.RefreshItemTooltip` (`self.MyTooltipWidget`) true _returnvalue true)
      (`SceneComponent.SetVisibility` (`self.Widget`) true false)
      (if _returnvalue
        ;[1 1 1] Send Current Actor to Char via Interface
        (message `/Game/TalentTreeBuilder/Blueprints/I_HeroUseItem.Hero_ItemToInteract` OtherActor self)))))

(fn `UserConstructionScript`
  (`parent.UserConstructionScript`))