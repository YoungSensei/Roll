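; Base pickup item actor for the Talent Tree Builder bonus examples, with an empty ItemUse event for children to implement.
; It builds a tooltip widget from its item data at BeginPlay, shown while overlapped.
; On overlap it queries the hero through interface messages to check class, level and item unlocks, refreshing the tooltip.
; If all pass, it registers itself as the hero's interaction item, clearing that when overlap ends.
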(event `self.ReceiveBeginPlay`
  (bind _returnvalue (`|CreateWidget` "/Game/TalentTreeBuilder/UI/BonusWidgets/W_ItemTooltip.W_ItemTooltip_C" null (`self.ItemIcon`) (`KismetTextLibrary.Conv_NameToText` (`self.ItemName`)) (`self.ItemType`) (`self.Required_Level`) (`self.Required_Talent`) (`self.ItemDescription`) (`self.ItemQualityColor`) (`self.Required_Class`)))
  (bind _output_get (set `self.MyTooltipWidget` _returnvalue))
  (`WidgetComponent.SetWidget` (`self.Widget`) _output_get))

(event `/Game/TalentTreeBuilder/Blueprints/I_InteractableItem.Item_Use`
  (params (UserSelfNode :type "Actor Object Reference"))
  ;[1 1 1] Here is empty, but used by children
)

(event `self.Collision.OnComponentBeginOverlap`
  (params (OverlappedComponent :type "PrimitiveComponent Object Reference") (OtherActor :type "Actor Object Reference") (OtherComp :type "PrimitiveComponent Object Reference") (OtherBodyIndex :type Integer) (bFromSweep :type Boolean) (SweepResult :type "HitResult Structure (by ref)"))
  (bind _output_get (set `self.CharRef` OtherActor))
  (`/Game/TalentTreeBuilder/Blueprints/LibMacroTalentSystem.CheckHeroTalentInterface` _output_get
    (:`true`
      ;[1 1 1] Check : Item Unlocked
      (bind _items (message `/Game/TalentTreeBuilder/Blueprints/I_HeroTalents.GetHero_UnlockedItems` (`self.CharRef`)))
      (bind _itemtypeslist (message `/Game/TalentTreeBuilder/Blueprints/I_HeroTalents.GetHero_UnlockedItemTypes` (`self.CharRef`)))
      ;[1 1 1] Check : Level and Class
      (bind _currentlevel (message `/Game/TalentTreeBuilder/Blueprints/I_HeroTalents.GetHero_Level` (`self.CharRef`)))
      (bind _class (message `/Game/TalentTreeBuilder/Blueprints/I_HeroTalents.GetHero_Class` (`self.CharRef`)))
      (bind _returnvalue (select `bool` (`|EnumEquality` (`self.Required_Class`) "NewEnumerator5") :`false` (`|EnumEquality` _class (`self.Required_Class`)) :`true` true))
      (bind _returnvalue_2 (>= _currentlevel (`self.Required_Level`)))
      (bind _returnvalue_3 (or (`KismetArrayLibrary.Array_Contains` _itemtypeslist (`self.ItemType`)) (`KismetArrayLibrary.Array_Contains` _items (`self.ItemName`))))
      (`/Game/TalentTreeBuilder/UI/BonusWidgets/W_ItemTooltip.RefreshItemTooltip` (`self.MyTooltipWidget`) _returnvalue _returnvalue_2 _returnvalue_3)
      ;[1 1 1] Show Tooltip
      (`SceneComponent.SetVisibility` (`self.Widget`) true false)
      ;[1 1 1] All requirements are Ok
      (if (and _returnvalue _returnvalue_2 _returnvalue_3)
        ;[1 1 1] Set ItemReferenceData to Character Via Interface
        (message `/Game/TalentTreeBuilder/Blueprints/I_HeroUseItem.Hero_ItemToInteract` (`self.CharRef`) self)))))

(event `self.Collision.OnComponentEndOverlap`
  (params (OverlappedComponent :type "PrimitiveComponent Object Reference") (OtherActor :type "Actor Object Reference") (OtherComp :type "PrimitiveComponent Object Reference") (OtherBodyIndex :type Integer))
  (`SceneComponent.SetVisibility` (`self.Widget`) false false)
  ;[1 1 1] Set to NONE ItemReferenceData to Character Via Interface
  (message `/Game/TalentTreeBuilder/Blueprints/I_HeroUseItem.Hero_ItemToInteract` (`self.CharRef`) null))

(fn `Item_GetData`
  (returns (ItemName :type Name) (ItemType :type "/Game/TalentTreeBuilder/Blueprints/E_ItemTypes Enum"))
  (return (`self.ItemName`) (`self.ItemType`)))

(fn `UserConstructionScript`)