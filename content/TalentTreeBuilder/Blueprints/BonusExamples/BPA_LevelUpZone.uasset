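; BPA_LevelUpZone is a bonus example actor from TalentTreeBuilder that levels up a character standing inside its collision zone.
; On overlap, the server stores the overlapping actor and starts a short looping timer that repeatedly sends it the HeroLevelUpMessage interface call.
; When any overlap ends, the server clears that reference and stops the timer, so the zone tracks only one actor at a time.
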(event `self.Collision.OnComponentBeginOverlap`
  (params (OverlappedComponent :type "PrimitiveComponent Object Reference") (OtherActor :type "Actor Object Reference") (OtherComp :type "PrimitiveComponent Object Reference") (OtherBodyIndex :type Integer) (bFromSweep :type Boolean) (SweepResult :type "HitResult Structure (by ref)"))
  (`/Engine/EditorBlueprintResources/ActorMacros.Switch Has Authority`
    (:`Authority`
      (set `self.CharRef` OtherActor)
      (bind _returnvalue (`KismetSystemLibrary.K2_SetTimerDelegate` (delegate `TickingLevelup`) 0.3 true))
      (set `self.Timer` _returnvalue))))

(event `TickingLevelup`
  ;[1 1 1] Send Command via Interface to LevelUp
  (message `/Game/TalentTreeBuilder/Blueprints/I_HeroUseItem.Hero_LevelUp` (`self.CharRef`)))

(event `self.Collision.OnComponentEndOverlap`
  (params (OverlappedComponent :type "PrimitiveComponent Object Reference") (OtherActor :type "Actor Object Reference") (OtherComp :type "PrimitiveComponent Object Reference") (OtherBodyIndex :type Integer))
  (`/Engine/EditorBlueprintResources/ActorMacros.Switch Has Authority`
    (:`Authority`
      ;[1 1 1] Forget Character and clear timer
      (set `self.CharRef` null)
      (`KismetSystemLibrary.K2_ClearAndInvalidateTimerHandle` (`self.Timer`)))))

(fn `UserConstructionScript`)