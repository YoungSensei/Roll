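; Pain zone actor that deals repeated damage to an overlapping actor and leaves it burning briefly after it exits.
; On the server, overlap begin stores the actor and starts a looping one-second damage timer.
; When that actor exits, a fire effect attaches to its mesh if it is a Character, and damage continues through a short delay before the timer clears.
; Only one target is tracked, so each new overlap overwrites it.
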(event `self.Collision.OnComponentBeginOverlap`
  (params (OverlappedComponent :type "PrimitiveComponent Object Reference") (OtherActor :type "Actor Object Reference") (OtherComp :type "PrimitiveComponent Object Reference") (OtherBodyIndex :type Integer) (bFromSweep :type Boolean) (SweepResult :type "HitResult Structure (by ref)"))
  (`/Engine/EditorBlueprintResources/ActorMacros.Switch Has Authority`
    (:`Authority`
      (set `self.CharRef` OtherActor)
      (bind _returnvalue (`KismetSystemLibrary.K2_SetTimerDelegate` (delegate `TickingDamage`) 1.0 true))
      (set `self.Timer` _returnvalue))))

(event `TickingDamage`
  (`GameplayStatics.ApplyDamage` (`self.CharRef`) (`self.Damage`)))

(event `self.Collision.OnComponentEndOverlap`
  (params (OverlappedComponent :type "PrimitiveComponent Object Reference") (OtherActor :type "Actor Object Reference") (OtherComp :type "PrimitiveComponent Object Reference") (OtherBodyIndex :type Integer))
  (`/Engine/EditorBlueprintResources/ActorMacros.Switch Has Authority`
    (:`Authority`
      (if (== OtherActor (`self.CharRef`))
        (bind _ascharacter (cast `Character` (`self.CharRef`)) ; ANY CHARACTER CLASS
          (:`then`
            (bind _returnvalue (`|SpawnActorFromClass` "/Game/TalentTreeBuilder/Blueprints/BonusExamples/BPA_Effect.BPA_Effect_C" (`KismetMathLibrary.MakeTransform` (0.0 0.0 0.0)) "AlwaysSpawn" "OverrideRootScale" null "/Game/TalentTreeBuilder/UnnecessaryContent/Particles/FX_Ambient/Fire/P_Fire_Book.P_Fire_Book" 3.0))
            (`self.K2_AttachToComponent` _returnvalue (`Character.Mesh` _ascharacter) "None" "SnapToTarget" "SnapToTarget" "SnapToTarget" true))
          (:`CastFailed`
            _))
        (`KismetSystemLibrary.Delay` 3.0)
        (`KismetSystemLibrary.K2_ClearAndInvalidateTimerHandle` (`self.Timer`))
        (set `self.CharRef` null)))))

(fn `UserConstructionScript`)