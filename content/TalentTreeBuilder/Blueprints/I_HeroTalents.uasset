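; Blueprint interface for heroes in the Talent Tree Builder, defining how other code reads and changes a hero's talents.
; Getters expose class, level, learned talents, free points, and unlocked items and item types.
; Mutators create or reset the talent set, set or add free points, and learn or reset single talents by data table ID or learned index, with flags for point accounting.
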(fn `AddHero_FreePoints`
  (params (Amount :type Integer)))

(fn `CreateHero_Talents`
  (params (LearnedTalents :type "Array of /Game/TalentTreeBuilder/Blueprints/S_LearnedTalentData Structure")))

(fn `GetHero_Class`
  (returns (Class :type "/Game/TalentTreeBuilder/Blueprints/E_HeroClasses Enum"))
  (return "NewEnumerator0"))

(fn `GetHero_FreePoints`
  (returns (CurrentFreePoints :type Integer))
  (return 0))

(fn `GetHero_Level`
  (returns (CurrentLevel :type Integer))
  (return 0))

(fn `GetHero_Talents`
  (returns (LearnedTalents :type "Array of /Game/TalentTreeBuilder/Blueprints/S_LearnedTalentData Structure"))
  (return))

(fn `GetHero_UnlockedItems`
  (returns (Items :type "Array of Name"))
  (return))

(fn `GetHero_UnlockedItemTypes`
  (returns (ItemTypesList :type "Array of /Game/TalentTreeBuilder/Blueprints/E_ItemTypes Enum"))
  (return))

(fn `LearnTalent_ByDataTableID`
  (params (TalentIndex :type Name) (DoNotDecreaseTalentPoints :type Boolean)))

(fn `LearnTalent_ByLearnedIndex`
  (params (IndexInLearnedTalents :type Integer) (DoNotDecreaseTalentPoints :type Boolean)))

(fn `ResetHero_Talents`)

(fn `ResetTalent_ByLearnedIndex`
  (params (IndexInLearnedTalents :type Integer) (RecalculateSpentPoints :type Boolean)))

(fn `SetHero_FreePoints`
  (params (FreePoints :type Integer)))