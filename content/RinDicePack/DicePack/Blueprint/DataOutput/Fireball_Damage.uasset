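; Fireball damage readout actor that shows the combined result of eight six-sided numbered dice on a text component.
; Every tick it casts eight dice references, picked from the level, to the D6 numbered dice Blueprint, sums their result values and writes the total as text.
; The update stops if any one of the eight casts fails.
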(event `self.ReceiveTick`
  (params (DeltaSeconds :type "Float (single-precision)"))
  ;[1 1 1] Read selected from level D6_NumDice Data
  (bind _asd6_num_dice_bp (cast `/Game/RinDicePack/D6_Num_Dice_BP` (`self.DiceToCheck`)))
  (bind _asd6_num_dice_bp_2 (cast `/Game/RinDicePack/D6_Num_Dice_BP` (`self.DiceToCheck2`)))
  (bind _asd6_num_dice_bp_3 (cast `/Game/RinDicePack/D6_Num_Dice_BP` (`self.DiceToCheck3`)))
  (bind _asd6_num_dice_bp_4 (cast `/Game/RinDicePack/D6_Num_Dice_BP` (`self.DiceToCheck4`)))
  (bind _asd6_num_dice_bp_5 (cast `/Game/RinDicePack/D6_Num_Dice_BP` (`self.DiceToCheck5`)))
  (bind _asd6_num_dice_bp_6 (cast `/Game/RinDicePack/D6_Num_Dice_BP` (`self.DiceToCheck6`)))
  (bind _asd6_num_dice_bp_7 (cast `/Game/RinDicePack/D6_Num_Dice_BP` (`self.DiceToCheck7`)))
  (bind _asd6_num_dice_bp_8 (cast `/Game/RinDicePack/D6_Num_Dice_BP` (`self.DiceToCheck8`)))
  (`TextRenderComponent.SetText` (`self.DataValue`) (`KismetStringLibrary.Conv_IntToString` (+ (`/Game/RinDicePack/D6_Num_Dice_BP.DiceResultData` _asd6_num_dice_bp) (`/Game/RinDicePack/D6_Num_Dice_BP.DiceResultData` _asd6_num_dice_bp_2) (`/Game/RinDicePack/D6_Num_Dice_BP.DiceResultData` _asd6_num_dice_bp_3) (`/Game/RinDicePack/D6_Num_Dice_BP.DiceResultData` _asd6_num_dice_bp_4) (`/Game/RinDicePack/D6_Num_Dice_BP.DiceResultData` _asd6_num_dice_bp_5) (`/Game/RinDicePack/D6_Num_Dice_BP.DiceResultData` _asd6_num_dice_bp_6) (`/Game/RinDicePack/D6_Num_Dice_BP.DiceResultData` _asd6_num_dice_bp_7) (`/Game/RinDicePack/D6_Num_Dice_BP.DiceResultData` _asd6_num_dice_bp_8)))))

(fn `UserConstructionScript`)